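; Route guide actor that shows a navigation path from the player to their chosen map destination while minimap mode and routing are active.
; A looping timer finds the navmesh path, feeds it to a spline and redraws it as short-lived debug arrows.
; It also shows a fast-travel widget, then on arrival ends the route and briefly displays a destination-reached widget unless fast travel was used.
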(event `self.ReceiveBeginPlay`
  (`KismetSystemLibrary.K2_SetTimerDelegate` (delegate `Ruta`) 0.1 true))

(event `Ruta`
  (bind _aspersonaje (cast `/Game/Blueprints/personaje` (`GameplayStatics.GetPlayerPawn` 0)))
  (if (and (`/Game/Blueprints/personaje.Mini` _aspersonaje) (`/Game/Blueprints/personaje.IniciaRuta` _aspersonaje))
    (`|ExecutionSequence`
      (:`then_0`
        (`GameplayStatics.GetActorOfClass` "/Game/Blueprints/personaje.personaje_C")
        (if (not (`self.isActive`))
          (bind _returnvalue (`|CreateWidget` "/Game/Widgets_recorrido/Recorrido/ViajeRapido.ViajeRapido_C" (`GameplayStatics.GetPlayerController` 0)))
          (bind _output_get (set `self.Viaje` _returnvalue))
          (`UserWidget.AddToViewport` _output_get 0)
          (set `self.isActive` true)))
      (:`then_1`
        (bind _returnvalue_2 (`NavigationSystemV1.FindPathToLocationSynchronously` (+ (`self.K2_GetActorLocation` _aspersonaje) (0.0 0.0 10.0)) (+ (`/Game/Blueprints/personaje.MouseLocationn` _aspersonaje) (0.0 0.0 10.0)) null null))
        (bind _pathpoints (`NavigationPath.PathPoints` _returnvalue_2))
        (`SplineComponent.SetSplinePoints` (`self.Spline`) _pathpoints "World" true)
        (for (_array_element _array_index) _pathpoints
          (if (!= _array_index 0)
            (`KismetSystemLibrary.DrawDebugArrow` (`|GetArrayItem` _pathpoints (- _array_index 1)) _array_element 200.0 (struct :`B` 1.0 :`A` 1.0) 0.1 20.0)
            (bind _aspersonaje_2 (cast `/Game/Blueprints/personaje` (`GameplayStatics.GetPlayerPawn` 0)))
            (bind (_returnvalue_x _returnvalue_y) (`KismetMathLibrary.BreakVector` (`self.K2_GetActorLocation` _aspersonaje_2)))
            (bind (_mouselocationn_x _mouselocationn_y) (`KismetMathLibrary.BreakVector` (`/Game/Blueprints/personaje.MouseLocationn` _aspersonaje_2)))
            (if (and (<= (`KismetMathLibrary.Abs` (- _returnvalue_x _mouselocationn_x)) 100.0) (<= (`KismetMathLibrary.Abs` (- _returnvalue_y _mouselocationn_y)) 100.0))
              (set `/Game/Blueprints/personaje.IniciaRuta` false _aspersonaje_2)
              (if (`/Game/Blueprints/personaje.isUsingViajeR` _aspersonaje_2)
                (set `/Game/Blueprints/personaje.isUsingViajeR` false _aspersonaje_2)
                (set `self.isActive` false)
                (else
                  (bind _returnvalue_3 (`|CreateWidget` "/Game/Widgets_recorrido/Recorrido/DestinoAlcanzado.DestinoAlcanzado_C" (`GameplayStatics.GetPlayerController` 0)))
                  (`UserWidget.AddToViewport` _returnvalue_3 0)
                  (`Widget.RemoveFromParent` _returnvalue)
                  (`KismetSystemLibrary.Delay` 2.0)
                  (`Widget.RemoveFromParent` _returnvalue_3)
                  (set `self.isActive` false))))))))
    (elif (`self.isActive`)
      (`Widget.RemoveFromParent` (`self.Viaje`))
      (set `self.isActive` false))))

(fn `UserConstructionScript`)