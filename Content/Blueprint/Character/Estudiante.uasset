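; Player character (student) for exploring buildings, with compass, pause menu, fast-travel map and a timed intro widget sequence before movement unlocks.
; Handles walk, run and jump, with looping timers for footsteps and speed-based camera shake.
; A toggled zoomable overhead camera lets the capsule overlap WorldStatic, restoring the last recorded overlap location on return.
; Camera traces tint the aimed object's material yellow; clicking sets location text and plays the matching building audio.
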(event `self.K2_OnMovementModeChanged`
  (params (PrevMovementMode :type "EMovementMode Enum" :default "MOVE_None") (NewMovementMode :type "EMovementMode Enum" :default "MOVE_None") (PrevCustomMode :type Byte) (NewCustomMode :type Byte))
  ;[1 1 1] Sonido caminando
  (if (and (`|EnumEquality` PrevMovementMode "MOVE_Falling") (`|EnumEquality` NewMovementMode "MOVE_Walking"))
    (`self.Pasos`)))

(event `InputAxis|Movimiento Y`
  (params (AxisValue :type "Float (single-precision)"))
  (bind (_returnvalue_x _returnvalue_y _returnvalue_z) (`KismetMathLibrary.BreakVector` (`self.GetVelocity`)))
  ;[1 1 1] Sonido caminando
  ;;[1 1 1] Control Teclado - Personaje
  (`self.AddMovementInput` (`KismetMathLibrary.GetRightVector` (`self.GetControlRotation`)) AxisValue)
  (if (and (or (!= _returnvalue_x 0.0) (!= _returnvalue_y 0.0)) (== _returnvalue_z 0.0) (== (`self.CamaraCenitalSonido`) (`self.Igual`)) (== (`self.Corriendo`) (`self.Igual`))) :!label _label
    (set `self.Caminando` true)
    (`/Engine/EditorBlueprintResources/StandardMacros.DoOnce` false :!label _label_2
      (:`Completed`
        (bind _returnvalue (`KismetSystemLibrary.K2_SetTimerDelegate` (delegate `Pasos`) 0.5 true))))
    (else
      (set `self.Caminando` false)
      (`KismetSystemLibrary.K2_ClearAndInvalidateTimerHandle` _returnvalue)
      (goto _label_2 :!via `Reset`))))

(event `Pasos`
  ;[1 1 1] Sonido caminando
  (`GameplayStatics.PlaySoundAtLocation` "/Game/Audios/Ambiente/PasosPiso__1_.PasosPiso__1_" (- (`self.K2_GetActorLocation`) (0.0 0.0 0.0)) (struct) 1.0 1.0 0.0 null null null null))

(event `Camera Shake Event`
  (bind _returnvalue (`GameplayStatics.GetPlayerController` 0))
  ;[1 1 1] Camera Shake
  (if (<= (`KismetMathLibrary.VSize` (`self.GetVelocity`)) 0.0)
    (if (`self.CamaraCenital1`)
      (`PlayerController.ClientStartCameraShake` :`self` _returnvalue :`Shake` "/Game/Blueprint/Camera/CameraShakeIdol.CameraShakeIdol_C"))
    (elif (`self.CamaraCenital1`)
      (`PlayerController.ClientStartCameraShake` :`self` _returnvalue :`Shake` "/Game/Blueprint/Camera/CameraShakeIdol1.CameraShakeIdol1_C"))))

(event `InputAxis|Movimiento X`
  (params (AxisValue :type "Float (single-precision)"))
  ;[1 1 1] Sonido caminando
  ;;[1 1 1] Control Teclado - Personaje
  (`self.AddMovementInput` (`KismetMathLibrary.GetForwardVector` (`self.GetControlRotation`)) AxisValue)
  (goto _label))

(event `self.ReceiveActorBeginOverlap`
  (params (OtherActor :type "Actor Object Reference"))
  ;[1 1 1] Capturar Cordenadas de Colision
  (if (not (`KismetStringLibrary.EqualEqual_StrStr` (`KismetSystemLibrary.GetDisplayName` OtherActor) "Landscape1"))
    (`KismetSystemLibrary.PrintString` "Hello")
    (set `self.COLISION` true)
    (set `self.LOCALIZACION_COLISION` (`SceneComponent.K2_GetComponentLocation` (`self.CapsuleComponent`)))))

(event `InputAxis|Vista X`
  (params (AxisValue :type "Float (single-precision)"))
  ;[1 1 1] Control Mouse - Personaje
  (`self.AddControllerYawInput` AxisValue))

(event `InputAxis|Vista Y`
  (params (AxisValue :type "Float (single-precision)"))
  ;[1 1 1] Control Mouse - Personaje
  (if (`self.CamaraCenital1`)
    (`self.AddControllerPitchInput` AxisValue)))

(event `self.ReceiveTick`
  (params (DeltaSeconds :type "Float (single-precision)"))
  (bind _returnvalue (`GameplayStatics.GetPlayerCameraManager` 0))
  (bind (_returnvalue_roll _returnvalue_pitch _returnvalue_yaw) (`KismetMathLibrary.BreakRotator` (`self.K2_GetActorRotation`)))
  (bind _index_poligonos (`self.INDEX POLIGONOS`))
  (bind _puntero_sprite1 (`self.Puntero_Sprite1`))
  (bind _returnvalue_2 (`self.K2_GetActorLocation` _returnvalue))
  ;[1 1 1] Distancia del Disparo
  ;;[1 1 1] Eventos permaentes
  (set `self.VarRotacionBrujula` _returnvalue_yaw)
  (`|ExecutionSequence`
    (:`then_0`
      (`self.Camera Shake Event`)
      (`SceneComponent.K2_SetWorldRotation` _puntero_sprite1 (`self.ROTACIÓN NORTE`) false false)
      (`SceneComponent.K2_SetWorldLocation` _puntero_sprite1 (- (`SceneComponent.K2_GetComponentLocation` (`self.SceneCaptureComponent2D`)) (0.0 1000.0 0.0)) false false)
      (bind _outactors (`GameplayStatics.GetAllActorsOfClass` "/Script/Landscape.Landscape"))
      ;[1 1 1] Cambio de Material Para el cambio de color
      (bind (_outhit _returnvalue_3) (`KismetSystemLibrary.LineTraceSingle` _returnvalue_2 (+ _returnvalue_2 (* (`self.GetActorForwardVector` _returnvalue) 3000.0)) "TraceTypeQuery1" true _outactors))
      (if _returnvalue_3
        (set `self.PASADO COLISION` true)
        (if (not (`self.CAPTURA MATERIAL`))
          ;[1 1 1] Buscar Inxdex del material a cambiar
          (bind _values (`BlueprintMapLibrary.Map_Values` _index_poligonos))
          (set `self.INDEX MATERIAL` (`|GetArrayItem` _values (`BlueprintMapLibrary.Map_Find` _index_poligonos (`KismetSystemLibrary.GetDisplayName` (`.HitActor` (`GameplayStatics.BreakHitResult` _outhit))))))
          (bind _output_get (set `self.ACTOR COLISION` (`.HitComponent` (`GameplayStatics.BreakHitResult` _outhit))))
          (bind _output_get_2 (set `self.MATERIAL OLD` (`PrimitiveComponent.GetMaterial` _output_get 0)))
          (set `self.CAPTURA MATERIAL` true)
          (`KismetSystemLibrary.PrintString` (`KismetSystemLibrary.GetDisplayName` _output_get_2) false false)
          (`PrimitiveComponent.SetMaterial` _output_get (`self.INDEX MATERIAL`) "/Game/Assets/Escenario/muro/amarillo.amarillo"))
        (elif (`self.PASADO COLISION`)
          (`PrimitiveComponent.SetMaterial` (`self.ACTOR COLISION`) (`self.INDEX MATERIAL`) (`self.MATERIAL OLD`))
          (set `self.CAPTURA MATERIAL` false))))))

(event `InputAction|Cambiar Camara`
  (params (Key :type "Key Structure"))
  (bind _capsulecomponent (`self.CapsuleComponent`))
  ;[1 1 1] Llamado Cambio de camaras
  (:`Pressed`
    (`/Engine/EditorBlueprintResources/StandardMacros.FlipFlop`
      (:`A`
        (`ActorComponent.Activate` (`self.CameraCenital`) false)
        (set `self.CamaraCenital1` false)
        (set `self.CamaraCenitalSonido` true)
        ;[1 1 1] Sistema de Colision dehabilitar y habilitar
        (`PrimitiveComponent.SetCollisionResponseToChannel` _capsulecomponent "ECC_WorldStatic" "ECR_Overlap")
        (if (`self.Press`)
          (`KismetSystemLibrary.K2_ClearAndInvalidateTimerHandle` (stale `Key|LeftShift` _returnvalue))))
      (:`B`
        (`ActorComponent.Deactivate` (`self.CameraCenital`))
        (set `self.CamaraCenital1` true)
        (set `self.CamaraCenitalSonido` false)
        (`PrimitiveComponent.SetCollisionResponseToChannel` _capsulecomponent "ECC_WorldStatic" "ECR_Block")
        (if (`self.COLISION`)
          (`SceneComponent.K2_SetWorldLocation` _capsulecomponent (`self.LOCALIZACION_COLISION`) false false)
          (set `self.COLISION` false))))))

(event `CustomEvent`
  ;[1 1 1] Sonido corriendo
  (`GameplayStatics.PlaySoundAtLocation` "/Game/Audios/Ambiente/PasosPiso__1_.PasosPiso__1_" (- (`self.K2_GetActorLocation`) (0.0 0.0 0.0)) (struct) 1.0 1.0 0.0 null null null null))

(event `Key|LeftShift`
  (params (Key :type "Key Structure"))
  (bind _charactermovement (`self.CharacterMovement`))
  (bind _camaracenital1 (`self.CamaraCenital1`))
  ;[1 1 1] Correr
  (:`Pressed`
    (set `self.Press` true)
    (if _camaracenital1
      (set `CharacterMovementComponent.MaxWalkSpeed` 1000.0 _charactermovement)
      ;[1 1 1] Sonido corriendo
      (set `self.Corriendo` true)
      (if (and (`self.Corriendo`) (`self.Mov`) (`self.CamaraCenital1`))
        (`/Engine/EditorBlueprintResources/StandardMacros.DoOnce` false :!label _label_3
          (:`Completed`
            (bind _returnvalue (`KismetSystemLibrary.K2_SetTimerDelegate` (delegate `CustomEvent`) 0.4 true))))
        (else
          (`KismetSystemLibrary.K2_ClearAndInvalidateTimerHandle` _returnvalue :!label _label_4)
          (goto _label_3 :!via `Reset`)))
      (else
        (set `CharacterMovementComponent.MaxWalkSpeed` 10000000000.0 _charactermovement)
        (`KismetSystemLibrary.K2_ClearAndInvalidateTimerHandle` _returnvalue))))
  (:`Released`
    (set `self.Press` false)
    (if _camaracenital1
      (set `CharacterMovementComponent.MaxWalkSpeed` 500.0 _charactermovement)
      (set `self.Corriendo` false)
      (if (not (`self.Corriendo`))
        (goto _label_4))
      (else
        (set `CharacterMovementComponent.MaxWalkSpeed` 1500.0 _charactermovement)
        (`KismetSystemLibrary.K2_ClearAndInvalidateTimerHandle` _returnvalue)))))

(event `InputAction|Saltar`
  (params (Key :type "Key Structure"))
  ;[1 1 1] Saltar
  (:`Pressed`
    (`self.Jump`)
    (set `self.Saltar` false))
  (:`Released`
    (`self.StopJumping`)
    (set `self.Saltar` true)))

(event `Key|MouseScrollUp`
  (params (Key :type "Key Structure"))
  (bind _cameracenital (`self.CameraCenital`))
  ;[1 1 1] Alejar Camara
  (:`Pressed`
    (`SceneComponent.K2_SetWorldLocation` _cameracenital (+ (0.0 0.0 1000.0) (`SceneComponent.K2_GetComponentLocation` _cameracenital)) false false)))

(event `Key|MouseScrollDown`
  (params (Key :type "Key Structure"))
  ;[1 1 1] Alejar Camara
  (:`Pressed`
    (if (< (`self.ALTURA INICIAL CAMARA`) (`KismetMathLibrary.FTrunc` (.z (`SceneComponent.K2_GetComponentLocation` (`self.CameraCenital`)))))
      (`SceneComponent.K2_SetWorldLocation` (`self.CameraCenital`) (- (`SceneComponent.K2_GetComponentLocation` (`self.CameraCenital`)) (0.0 0.0 1000.0)) false false))))

(event `Key|LeftMouseButton`
  (params (Key :type "Key Structure"))
  (bind _returnvalue (`GameplayStatics.GetPlayerCameraManager` 0))
  (bind _returnvalue_2 (`self.K2_GetActorLocation` _returnvalue))
  ;[1 1 1] Llamado Rayo Colisionador
  (:`Pressed`
    (bind _outactors (`GameplayStatics.GetAllActorsOfClass` "/Script/Landscape.Landscape"))
    (bind (_outhit _returnvalue_3) (`KismetSystemLibrary.LineTraceSingle` _returnvalue_2 (+ _returnvalue_2 (* (`self.GetActorForwardVector` _returnvalue) 50000.0)) "TraceTypeQuery1" false _outactors))
    (if _returnvalue_3
      (bind _returnvalue_4 (`KismetSystemLibrary.GetDisplayName` (`.HitActor` (`GameplayStatics.BreakHitResult` _outhit))))
      ;[1 1 1] Actualizar variable para la ubicación del jugador
      (set `self.Ubicacion` (`KismetStringLibrary.Replace` (`KismetStringLibrary.Concat_StrStr` "Se encuentra en " _returnvalue_4) "_" " "))
      ;[1 1 1] Busqueda de Audio con Comparación de Nombre
      (for _array_element (`self.NOMBRES_EDIFICIOS`)
        (set `self.IGUALDAD` (`KismetStringLibrary.EqualEqual_StrStr` _returnvalue_4 _array_element))
        (set `self.INDICE` (`KismetArrayLibrary.Array_Find` (`self.NOMBRES_EDIFICIOS`) _returnvalue_4))
        (if (`self.IGUALDAD`)
          (`KismetSystemLibrary.Delay` 0.2)
          (`GameplayStatics.PlaySound2D` (`|GetArrayItem` (`self.SONIDO_EDIFICIOS`) (`self.INDICE`)) 1.0 1.0 0.0 null null)
          (`KismetSystemLibrary.Delay` 5.0)
          (set `self.Ubicacion` ""))))))

(event `InputAction|Menu Pausa`
  (params (Key :type "Key Structure"))
  (bind _returnvalue (`GameplayStatics.GetPlayerController` 0))
  ;[1 1 1] Llamado Menu Pausa
  (:`Pressed`
    (if (`self.BCameraW`)
      (bind _returnvalue_2 (`|CreateWidget` "/Game/Blueprint/Widgets/MenuPausa.MenuPausa_C"))
      (bind _output_get (set `self.MenuPausa` _returnvalue_2))
      (`UserWidget.AddToPlayerScreen` _output_get 0)
      ;;[1 1 1] Bloquear Movimiento de personaje y mostrar Mouse
      (`WidgetBlueprintLibrary.SetInputMode_UIOnlyEx` _returnvalue _returnvalue_2)
      (set `PlayerController.bShowMouseCursor` true _returnvalue))))

(event `InputAction|Abrir Mapa`
  (params (Key :type "Key Structure"))
  (bind _returnvalue (`GameplayStatics.GetPlayerController` 0))
  ;[1 1 1] Llamado Mapa Viaje Rapido
  (:`Pressed`
    (if (`self.BCameraW`)
      (bind _returnvalue_2 (`|CreateWidget` "/Game/HUDS/Campus/Mapa.Mapa_C" _returnvalue))
      (`UserWidget.AddToPlayerScreen` _returnvalue_2 0)
      (`WidgetBlueprintLibrary.SetInputMode_UIOnlyEx` _returnvalue _returnvalue_2)
      (set `PlayerController.bShowMouseCursor` true _returnvalue))))

(event `self.ReceiveBeginPlay`
  ;[1 1 1] Llamado HUD
  (`CharacterMovementComponent.DisableMovement` (`self.CharacterMovement`))
  (bind _returnvalue (`|CreateWidget` "/Game/Blueprint/Widgets/Inicio/WInicio.WInicio_C" (`GameplayStatics.GetPlayerController` 0)))
  (bind _output_get (set `self.Inicio` _returnvalue))
  (`UserWidget.AddToPlayerScreen` _output_get 0)
  ;[1 1 1] Extraer Rotación Inicial del Norte
  (set `self.ROTACIÓN NORTE` (`SceneComponent.K2_GetComponentRotation` (`self.Puntero_Sprite1`)))
  ;[1 1 1] Valor Inicial de Variable
  (set `self.ACTOR COLISION` (`self.Mesh`))
  ;[1 1 1] Letreros de instrucciones
  (`KismetSystemLibrary.ExecuteConsoleCommand` "t.maxfps 300" null)
  (`KismetSystemLibrary.Delay` 5.0)
  (`WidgetLayoutLibrary.RemoveAllWidgets`)
  (bind _returnvalue_2 (`|CreateWidget` "/Game/Blueprint/Widgets/Inicio/WMoverse.WMoverse_C"))
  (bind _output_get_2 (set `self.Movimiento` _returnvalue_2))
  (`UserWidget.AddToPlayerScreen` _output_get_2 0)
  (`KismetSystemLibrary.Delay` 5.0)
  (`WidgetLayoutLibrary.RemoveAllWidgets`)
  (bind _returnvalue_3 (`|CreateWidget` "/Game/Blueprint/Widgets/Inicio/WCorrer.WCorrer_C"))
  (bind _output_get_3 (set `self.WCorrer` _returnvalue_3))
  (`UserWidget.AddToPlayerScreen` _output_get_3 0)
  (`KismetSystemLibrary.Delay` 5.0)
  (`WidgetLayoutLibrary.RemoveAllWidgets`)
  (bind _returnvalue_4 (`|CreateWidget` "/Game/Blueprint/Widgets/Inicio/WMapa.WMapa_C"))
  (bind _output_get_4 (set `self.Mapa` _returnvalue_4))
  (`UserWidget.AddToPlayerScreen` _output_get_4 0)
  (`KismetSystemLibrary.Delay` 5.0)
  (`WidgetLayoutLibrary.RemoveAllWidgets`)
  (bind _returnvalue_5 (`|CreateWidget` "/Game/Blueprint/Widgets/Inicio/WClic.WClic_C"))
  (bind _output_get_5 (set `self.Clic` _returnvalue_5))
  (`UserWidget.AddToPlayerScreen` _output_get_5 0)
  (`KismetSystemLibrary.Delay` 1.0)
  (`WidgetLayoutLibrary.RemoveAllWidgets`)
  (bind _returnvalue_6 (`|CreateWidget` "/Game/Blueprint/Widgets/Brujula_Superior.Brujula_Superior_C"))
  (`UserWidget.AddToPlayerScreen` _returnvalue_6 0)
  (bind _returnvalue_7 (`|CreateWidget` "/Game/Blueprint/Widgets/Camera_widget.Camera_widget_C"))
  (bind _output_get_6 (set `self.Camera Widget` _returnvalue_7))
  (`UserWidget.AddToPlayerScreen` _output_get_6 0)
  (set `self.BCameraW` true)
  (`CharacterMovementComponent.SetMovementMode` (`self.CharacterMovement`) "MOVE_Walking" 0)
  (set `self.Mov` true))

(fn `UserConstructionScript`)