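; Trigger box that lets the Estudiante character enter the Calle 100 interior level.
; Overlapping its Cube enables input on the actor and shows the InteractuarCalle100 prompt widget; leaving disables input and removes the widget.
; While input is enabled, pressing E opens CALLE100_INTERIOR by name.
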(event `Key|E`
  (params (Key :type "Key Structure"))
  (:`Pressed`
    (`GameplayStatics.OpenLevel` "CALLE100_INTERIOR")))

(event `self.Cube.OnComponentBeginOverlap`
  (params (OverlappedComponent :type "PrimitiveComponent Object Reference") (OtherActor :type "Actor Object Reference") (OtherComp :type "PrimitiveComponent Object Reference") (OtherBodyIndex :type Integer) (bFromSweep :type Boolean) (SweepResult :type "HitResult Structure (by ref)"))
  (cast `/Game/Blueprint/Character/Estudiante` OtherActor)
  (`self.EnableInput` (`GameplayStatics.GetPlayerController` 0))
  (bind _returnvalue (`|CreateWidget` "/Game/Blueprint/Widgets/InteractuarCalle100.InteractuarCalle100_C"))
  (`UserWidget.AddToViewport` _returnvalue 0))

(event `self.Cube.OnComponentEndOverlap`
  (params (OverlappedComponent :type "PrimitiveComponent Object Reference") (OtherActor :type "Actor Object Reference") (OtherComp :type "PrimitiveComponent Object Reference") (OtherBodyIndex :type Integer))
  (cast `/Game/Blueprint/Character/Estudiante` OtherActor)
  (`self.DisableInput` (`GameplayStatics.GetPlayerController` 0))
  (`Widget.RemoveFromParent` (stale `self.Cube.OnComponentBeginOverlap` _returnvalue)))

(fn `UserConstructionScript`)